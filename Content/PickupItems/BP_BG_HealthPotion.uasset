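; BP_BG_HealthPotion is a health pickup that heals the MainCharacter on overlap.
; Each Tick adds a small random yaw to the Potion component, so the spin is uneven and frame-rate dependent.
; A Sphere overlap sets its collision to query-only and, if health is below maximum, adds HealthToAdd capped at MaxHealth.
; The potion destroys itself only after healing, so it remains when health is full.
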(event OnComponentBeginOverlap(Sphere)
  (params (OverlappedComponent :type Primitive%20Component%20Object%20Reference) (OtherActor :type Actor%20Object%20Reference) (OtherComp :type Primitive%20Component%20Object%20Reference) (OtherBodyIndex :type Integer) (bFromSweep :type Boolean) (SweepResult :type Hit%20Result%20Structure%20%28by%20ref%29))
  ;[1 1 1] Pickup system
  (bind _asmain_character (Utilities|Casting|CastToMainCharacter OtherActor))
  (Collision|SetCollisionEnabled (Variables|Default|GetSphere) "QueryOnly")
  (if (< (Variables|/Game/MainCharacter/Player/Demo/ThirdPersonTemplate/ThirdPersonBP/Blueprints/MainCharacter.MainCharacter_C|GetHealth _asmain_character) (Variables|/Game/MainCharacter/Player/Demo/ThirdPersonTemplate/ThirdPersonBP/Blueprints/MainCharacter.MainCharacter_C|GetMaxHealth _asmain_character))
    (if (> (+ (Variables|/Game/MainCharacter/Player/Demo/ThirdPersonTemplate/ThirdPersonBP/Blueprints/MainCharacter.MainCharacter_C|GetHealth _asmain_character) (Variables|Default|GethealthToAdd)) (Variables|/Game/MainCharacter/Player/Demo/ThirdPersonTemplate/ThirdPersonBP/Blueprints/MainCharacter.MainCharacter_C|GetMaxHealth _asmain_character))
      (Variables|/Game/MainCharacter/Player/Demo/ThirdPersonTemplate/ThirdPersonBP/Blueprints/MainCharacter.MainCharacter_C|SetHealth _asmain_character (Variables|/Game/MainCharacter/Player/Demo/ThirdPersonTemplate/ThirdPersonBP/Blueprints/MainCharacter.MainCharacter_C|GetMaxHealth _asmain_character))
      (else
        (Variables|/Game/MainCharacter/Player/Demo/ThirdPersonTemplate/ThirdPersonBP/Blueprints/MainCharacter.MainCharacter_C|SetHealth _asmain_character (+ (Variables|/Game/MainCharacter/Player/Demo/ThirdPersonTemplate/ThirdPersonBP/Blueprints/MainCharacter.MainCharacter_C|GetHealth _asmain_character) (Variables|Default|GethealthToAdd)))))
    (Actor|DestroyActor)))

(event EventTick
  (params (DeltaSeconds :type Float%20%28single-precision%29))
  ;[1 1 1] Item rotation
  (Transformation|AddRelativeRotation (Variables|Default|GetPotion) (Math|Rotator|MakeRotator 0.0 0.0 (Math|Random|RandomFloatinRange 0.0 2.0)) false false))

(fn ConstructionScript)