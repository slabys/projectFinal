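; BP_SM_GoldChest is a gold pickup that grants gold to the MainCharacter and shows the amount above itself.
; Tick spins the Potion component by a small random yaw each frame.
; Overlapping Sphere adds GoldToAdd to the character's Gold, disables the sphere's collision and destroys the chest.
; A separate TextVisibilityCollision volume shows and hides a TextAbove widget with the gold amount as the character enters and leaves.
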(event OnComponentBeginOverlap(Sphere)
  (params (OverlappedComponent :type Primitive%20Component%20Object%20Reference) (OtherActor :type Actor%20Object%20Reference) (OtherComp :type Primitive%20Component%20Object%20Reference) (OtherBodyIndex :type Integer) (bFromSweep :type Boolean) (SweepResult :type Hit%20Result%20Structure%20%28by%20ref%29))
  ;[1 1 1] Pickup item
  (bind _asmain_character (Utilities|Casting|CastToMainCharacter OtherActor))
  (Collision|SetCollisionEnabled (Variables|Default|GetSphere) "NoCollision")
  (Variables|/Game/MainCharacter/Player/MainCharacter.MainCharacter_C|SetGold _asmain_character (+ (Variables|/Game/MainCharacter/Player/MainCharacter.MainCharacter_C|GetGold _asmain_character) (Variables|Default|GetgoldToAdd)))
  (Actor|DestroyActor))

(event OnComponentBeginOverlap(TextVisibilityCollision)
  (params (OverlappedComponent :type Primitive%20Component%20Object%20Reference) (OtherActor :type Actor%20Object%20Reference) (OtherComp :type Primitive%20Component%20Object%20Reference) (OtherBodyIndex :type Integer) (bFromSweep :type Boolean) (SweepResult :type Hit%20Result%20Structure%20%28by%20ref%29))
  ;[1 1 1] Text above item
  (Utilities|Casting|CastToMainCharacter OtherActor)
  (bind _astext_above (Utilities|Casting|CastToTextAbove (UserInterface|GetUserWidgetObject (Variables|Default|GetWidget))))
  (Widget|SetVisibility _astext_above "Visible")
  (Rendering|Components|TextRender|SetText (Variables|/Game/Characters/UI/TextAbove.TextAbove_C|GetTextAboveCharacter _astext_above) (Utilities|Text|ToText(String) (Utilities|String|Append "Gold: +" (Utilities|String|ToString(Integer) (Variables|Default|GetgoldToAdd))))))

(event OnComponentEndOverlap(TextVisibilityCollision)
  (params (OverlappedComponent :type Primitive%20Component%20Object%20Reference) (OtherActor :type Actor%20Object%20Reference) (OtherComp :type Primitive%20Component%20Object%20Reference) (OtherBodyIndex :type Integer))
  ;[1 1 1] Text above item
  (Utilities|Casting|CastToMainCharacter OtherActor)
  (bind _astext_above (Utilities|Casting|CastToTextAbove (UserInterface|GetUserWidgetObject (Variables|Default|GetWidget))))
  (Widget|SetVisibility _astext_above "Hidden"))

(event EventBeginPlay)

(event Collision|EventActorBeginOverlap
  (params (OtherActor :type Actor%20Object%20Reference)))

(event EventTick
  (params (DeltaSeconds :type Float%20%28single-precision%29))
  ;[1 1 1] Item rotation
  (Transformation|AddRelativeRotation (Variables|Default|GetPotion) (Math|Rotator|MakeRotator 0.0 0.0 (Math|Random|RandomFloatinRange 0.0 3.0)) false false))

(fn ConstructionScript)