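; Teleport scroll pickup, despite the HealthPotion asset name, that sets HasMagicScroll on the MainCharacter when it overlaps the Sphere, then destroys itself.
; A separate TextVisibilityCollision volume shows the TextAbove widget with a scroll hint while the MainCharacter is inside and hides it on exit.
; Tick spins the Scroll component by a small random yaw step each frame, so the rotation speed depends on frame rate.
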(event OnComponentBeginOverlap(Sphere)
  (params (OverlappedComponent :type Primitive%20Component%20Object%20Reference) (OtherActor :type Actor%20Object%20Reference) (OtherComp :type Primitive%20Component%20Object%20Reference) (OtherBodyIndex :type Integer) (bFromSweep :type Boolean) (SweepResult :type Hit%20Result%20Structure%20%28by%20ref%29))
  ;[1 1 1] Item pickup
  (bind _asmain_character (Utilities|Casting|CastToMainCharacter OtherActor))
  (Variables|/Game/MainCharacter/Player/ThirdPersonBP/Blueprints/MainCharacter.MainCharacter_C|SethasMagicScroll _asmain_character true)
  (Actor|DestroyActor))

(event OnComponentBeginOverlap(TextVisibilityCollision)
  (params (OverlappedComponent :type Primitive%20Component%20Object%20Reference) (OtherActor :type Actor%20Object%20Reference) (OtherComp :type Primitive%20Component%20Object%20Reference) (OtherBodyIndex :type Integer) (bFromSweep :type Boolean) (SweepResult :type Hit%20Result%20Structure%20%28by%20ref%29))
  (Utilities|Casting|CastToMainCharacter OtherActor)
  (bind _astext_above (Utilities|Casting|CastToTextAbove (UserInterface|GetUserWidgetObject (Variables|Default|GetWidget))))
  (Widget|SetVisibility _astext_above "Visible")
  (Rendering|Components|TextRender|SetText (Variables|/Game/Characters/UI/TextAbove.TextAbove_C|GetTextAboveCharacter _astext_above) "Teleport Scroll  
(Might be useful)"))

(event OnComponentEndOverlap(TextVisibilityCollision)
  (params (OverlappedComponent :type Primitive%20Component%20Object%20Reference) (OtherActor :type Actor%20Object%20Reference) (OtherComp :type Primitive%20Component%20Object%20Reference) (OtherBodyIndex :type Integer))
  (Utilities|Casting|CastToMainCharacter OtherActor)
  (bind _astext_above (Utilities|Casting|CastToTextAbove (UserInterface|GetUserWidgetObject (Variables|Default|GetWidget))))
  (Widget|SetVisibility _astext_above "Hidden"))

(event EventTick
  (params (DeltaSeconds :type Float%20%28single-precision%29))
  ;[1 1 1] Item rotation
  (Transformation|AddRelativeRotation (Variables|Default|GetScroll) (Math|Rotator|MakeRotator 0.0 0.0 (Math|Random|RandomFloatinRange 0.0 3.0)) false false))

(fn ConstructionScript)