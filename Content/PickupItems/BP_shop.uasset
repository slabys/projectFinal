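; Shop actor with an animated trader who greets the player and two purchasable gear items that boost stats.
; Item overlap boxes, gated by the player's ShopAreaOverlap flag, show price prompts and select the item.
; The Interaction input checks gold and ownership, then deducts the price, refreshes clothing and destroys the item component.
; The helmet raises health and max health, while hand armor raises base and critical damage.
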(event OnComponentBeginOverlap(TraderTrigger)
  (params (OverlappedComponent :type Primitive%20Component%20Object%20Reference) (OtherActor :type Actor%20Object%20Reference) (OtherComp :type Primitive%20Component%20Object%20Reference) (OtherBodyIndex :type Integer) (bFromSweep :type Boolean) (SweepResult :type Hit%20Result%20Structure%20%28by%20ref%29))
  ;[1 1 1] Trigger of trader :O
  (Utilities|Casting|CastToMainCharacter OtherActor)
  (bind _astext_above (Utilities|Casting|CastToTextAbove (UserInterface|GetUserWidgetObject (Variables|Default|GetTraderText))))
  (Widget|SetVisibility _astext_above "Visible")
  (Rendering|Components|TextRender|SetText (Variables|/Game/Characters/UI/TextAbove.TextAbove_C|GetTextAboveCharacter _astext_above) "Come and buy something! 
Get boost for your abilities.")
  (Components|Animation|PlayAnimation (Variables|Default|GetTrader) "/Game/Characters/Animations/Animations/TraderTrading.TraderTrading" false))

(event OnComponentEndOverlap(TraderTrigger)
  (params (OverlappedComponent :type Primitive%20Component%20Object%20Reference) (OtherActor :type Actor%20Object%20Reference) (OtherComp :type Primitive%20Component%20Object%20Reference) (OtherBodyIndex :type Integer))
  ;[1 1 1] Trigger of trader :O
  (Utilities|Casting|CastToMainCharacter OtherActor)
  (Components|Animation|PlayAnimation (Variables|Default|GetTrader) "/Game/Characters/Animations/Animations/TraderIdle.TraderIdle" true)
  (bind _astext_above (Utilities|Casting|CastToTextAbove (UserInterface|GetUserWidgetObject (Variables|Default|GetTraderText))))
  (Rendering|Components|TextRender|SetText (Variables|/Game/Characters/UI/TextAbove.TextAbove_C|GetTextAboveCharacter _astext_above) "See you later!")
  (Utilities|FlowControl|Delay 1e+01)
  (Widget|SetVisibility _astext_above "Hidden"))

(event OnComponentBeginOverlap(Item2Box)
  (params (OverlappedComponent :type Primitive%20Component%20Object%20Reference) (OtherActor :type Actor%20Object%20Reference) (OtherComp :type Primitive%20Component%20Object%20Reference) (OtherBodyIndex :type Integer) (bFromSweep :type Boolean) (SweepResult :type Hit%20Result%20Structure%20%28by%20ref%29))
  ;[1 1 1] Overlap item box 2
  (bind _asmain_character (Utilities|Casting|CastToMainCharacter OtherActor))
  (Variables|Default|SetisOverlapping true)
  (if (Variables|/Game/MainCharacter/Player/ThirdPersonBP/Blueprints/MainCharacter.MainCharacter_C|GetshopAreaOverlap _asmain_character)
    (bind _astext_above (Utilities|Casting|CastToTextAbove (UserInterface|GetUserWidgetObject (Variables|Default|GetItem2Widget))))
    (Widget|SetVisibility _astext_above "Visible")
    (Rendering|Components|TextRender|SetText (Variables|/Game/Characters/UI/TextAbove.TextAbove_C|GetTextAboveCharacter _astext_above) (Utilities|Text|ToText(String) (Utilities|String|Append "Hand armor - " (Utilities|String|ToString(Integer) (Variables|Default|GetitemTwoPrice)) " gold 
Press F to buy")))
    (Variables|Default|SetitemTwoSelected true)
    (Variables|Default|SetitemOneSelected false)))

(event OnComponentEndOverlap(Item2Box)
  (params (OverlappedComponent :type Primitive%20Component%20Object%20Reference) (OtherActor :type Actor%20Object%20Reference) (OtherComp :type Primitive%20Component%20Object%20Reference) (OtherBodyIndex :type Integer))
  ;[1 1 1] End ovelap of player and item
  (Utilities|Casting|CastToMainCharacter OtherActor)
  (bind _astext_above (Utilities|Casting|CastToTextAbove (UserInterface|GetUserWidgetObject (Variables|Default|GetItem2Widget))))
  (Widget|SetVisibility _astext_above "Hidden")
  (Variables|Default|SetitemOneSelected false)
  (Variables|Default|SetitemTwoSelected false)
  (Variables|Default|SetisOverlapping false))

(event OnComponentBeginOverlap(Item1Box)
  (params (OverlappedComponent :type Primitive%20Component%20Object%20Reference) (OtherActor :type Actor%20Object%20Reference) (OtherComp :type Primitive%20Component%20Object%20Reference) (OtherBodyIndex :type Integer) (bFromSweep :type Boolean) (SweepResult :type Hit%20Result%20Structure%20%28by%20ref%29))
  ;[1 1 1] Overlap box item 1
  (bind _asmain_character (Utilities|Casting|CastToMainCharacter OtherActor))
  (Variables|Default|SetisOverlapping true)
  (if (Variables|/Game/MainCharacter/Player/ThirdPersonBP/Blueprints/MainCharacter.MainCharacter_C|GetshopAreaOverlap _asmain_character)
    (bind _astext_above (Utilities|Casting|CastToTextAbove (UserInterface|GetUserWidgetObject (Variables|Default|GetItem1Widget))))
    (Widget|SetVisibility _astext_above "Visible")
    (Rendering|Components|TextRender|SetText (Variables|/Game/Characters/UI/TextAbove.TextAbove_C|GetTextAboveCharacter _astext_above) (Utilities|Text|ToText(String) (Utilities|String|Append "Helmet - " (Utilities|String|ToString(Integer) (Variables|Default|GetitemOnePrice)) " gold 
Press F to buy")))
    (Variables|Default|SetitemOneSelected true)
    (Variables|Default|SetitemTwoSelected false)))

(event OnComponentEndOverlap(Item1Box)
  (params (OverlappedComponent :type Primitive%20Component%20Object%20Reference) (OtherActor :type Actor%20Object%20Reference) (OtherComp :type Primitive%20Component%20Object%20Reference) (OtherBodyIndex :type Integer))
  ;[1 1 1] End ovelap of player and item
  (Utilities|Casting|CastToMainCharacter OtherActor)
  (bind _astext_above (Utilities|Casting|CastToTextAbove (UserInterface|GetUserWidgetObject (Variables|Default|GetItem1Widget))))
  (Widget|SetVisibility _astext_above "Hidden")
  (Variables|Default|SetitemOneSelected false)
  (Variables|Default|SetitemTwoSelected false)
  (Variables|Default|SetisOverlapping false))

(event Input|ActionEvents|InputActionInteraction
  (params (Key :type Key%20Structure :default "None"))
  (bind _returnvalue (Game|GetPlayerCharacter 0))
  (bind _returnvalue_2 (Game|GetPlayerCharacter 0))
  (bind _itemoneprice (Variables|Default|GetitemOnePrice))
  (bind _itemtwoprice (Variables|Default|GetitemTwoPrice))
  ;[1 1 1] BuyOverlaped item
  (:Pressed
    (bind _output_get (Variables|Default|SetisActionBuy true))
    (if (and _output_get (Variables|Default|GetisOverlapping))
      (Utilities|FlowControl|Sequence
        (:then_0
          (if (Variables|Default|GetitemOneSelected)
            (bind _asmain_character (Utilities|Casting|CastToMainCharacter _returnvalue_2))
            (if (and (!= (Variables|/Game/MainCharacter/Player/ThirdPersonBP/Blueprints/MainCharacter.MainCharacter_C|GetMaskVisibility _asmain_character) true) (>= (Variables|/Game/MainCharacter/Player/ThirdPersonBP/Blueprints/MainCharacter.MainCharacter_C|GetGold _asmain_character) _itemoneprice))
              (Variables|/Game/MainCharacter/Player/ThirdPersonBP/Blueprints/MainCharacter.MainCharacter_C|SetMaskVisibility _asmain_character true)
              (Default|RefreshClothing _asmain_character)
              (Variables|/Game/MainCharacter/Player/ThirdPersonBP/Blueprints/MainCharacter.MainCharacter_C|SetGold _asmain_character (- (Variables|/Game/MainCharacter/Player/ThirdPersonBP/Blueprints/MainCharacter.MainCharacter_C|GetGold _asmain_character) _itemoneprice))
              (Widget|SetVisibility (Variables|/Game/Characters/UI/TextAbove.TextAbove_C|GetTextAboveCharacter (stale OnComponentBeginOverlap(Item1Box) _astext_above)) "Hidden")
              (Components|DestroyComponent (Variables|Default|GetItem1))
              (Variables|Default|SetisOverlapping false)
              (Variables|Default|SetisActionBuy false)
              ;[1 1 1] Add health from adding armor
              (bind _asmain_character_2 (Utilities|Casting|CastToMainCharacter _returnvalue))
              (Utilities|FlowControl|Sequence
                (:then_0
                  (Variables|/Game/MainCharacter/Player/ThirdPersonBP/Blueprints/MainCharacter.MainCharacter_C|SetMaxHealth _asmain_character_2 (+ (Variables|/Game/MainCharacter/Player/ThirdPersonBP/Blueprints/MainCharacter.MainCharacter_C|GetMaxHealth _asmain_character_2) 50)))
                (:then_1
                  (Variables|/Game/MainCharacter/Player/ThirdPersonBP/Blueprints/MainCharacter.MainCharacter_C|SetHealth _asmain_character_2 (+ (Variables|/Game/MainCharacter/Player/ThirdPersonBP/Blueprints/MainCharacter.MainCharacter_C|GetHealth _asmain_character_2) 50))))
              (else
                (Rendering|Components|TextRender|SetText (Variables|/Game/Characters/UI/TextAbove.TextAbove_C|GetTextAboveCharacter (stale OnComponentBeginOverlap(Item1Box) _astext_above)) "Not enough gold mate!")
                (Widget|SetVisibility (Variables|/Game/Characters/UI/TextAbove.TextAbove_C|GetTextAboveCharacter (stale OnComponentBeginOverlap(Item1Box) _astext_above)) "Visible")
                (Variables|Default|SetisOverlapping false :!label _label)
                (Variables|Default|SetisActionBuy false)))))
        (:then_1
          (if (Variables|Default|GetitemTwoSelected) :!label _label_2
            (bind _asmain_character_3 (Utilities|Casting|CastToMainCharacter _returnvalue_2))
            (if (and (!= (Variables|/Game/MainCharacter/Player/ThirdPersonBP/Blueprints/MainCharacter.MainCharacter_C|GetArmorVisibility _asmain_character_3) true) (>= (Variables|/Game/MainCharacter/Player/ThirdPersonBP/Blueprints/MainCharacter.MainCharacter_C|GetGold _asmain_character_3) _itemtwoprice))
              (Variables|/Game/MainCharacter/Player/ThirdPersonBP/Blueprints/MainCharacter.MainCharacter_C|SetArmorVisibility _asmain_character_3 true)
              (Default|RefreshClothing _asmain_character_3)
              (Variables|/Game/MainCharacter/Player/ThirdPersonBP/Blueprints/MainCharacter.MainCharacter_C|SetGold _asmain_character_3 (- (Variables|/Game/MainCharacter/Player/ThirdPersonBP/Blueprints/MainCharacter.MainCharacter_C|GetGold _asmain_character_3) _itemtwoprice))
              (Widget|SetVisibility (Variables|/Game/Characters/UI/TextAbove.TextAbove_C|GetTextAboveCharacter (stale OnComponentBeginOverlap(Item2Box) _astext_above)) "Hidden")
              (Components|DestroyComponent (Variables|Default|GetItem2))
              (Variables|Default|SetisOverlapping false)
              (Variables|Default|SetisActionBuy false)
              ;[1 1 1] Add damage from hand armor
              (bind _asmain_character_4 (Utilities|Casting|CastToMainCharacter _returnvalue))
              (Utilities|FlowControl|Sequence
                (:then_0
                  (Variables|/Game/MainCharacter/Player/ThirdPersonBP/Blueprints/MainCharacter.MainCharacter_C|SetbaseDamage _asmain_character_4 (+ (Variables|/Game/MainCharacter/Player/ThirdPersonBP/Blueprints/MainCharacter.MainCharacter_C|GetbaseDamage _asmain_character_4) 2.0)))
                (:then_1
                  (Variables|/Game/MainCharacter/Player/ThirdPersonBP/Blueprints/MainCharacter.MainCharacter_C|SetbaseCriticalDamage _asmain_character_4 (+ (Variables|/Game/MainCharacter/Player/ThirdPersonBP/Blueprints/MainCharacter.MainCharacter_C|GetbaseCriticalDamage _asmain_character_4) 5.0))))
              (else
                (Rendering|Components|TextRender|SetText (Variables|/Game/Characters/UI/TextAbove.TextAbove_C|GetTextAboveCharacter (stale OnComponentBeginOverlap(Item2Box) _astext_above)) "Not enough gold mate!")
                (Widget|SetVisibility (Variables|/Game/Characters/UI/TextAbove.TextAbove_C|GetTextAboveCharacter (stale OnComponentBeginOverlap(Item2Box) _astext_above)) "Visible")
                (goto _label))))))
      (else
        (goto _label_2)))))

(fn ConstructionScript)