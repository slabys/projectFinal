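; Melee enemy Blueprint that detects the player via PawnSensing, chases, attacks, and dies when health runs out.
; Sightings refresh a ten-second awareness timer and, once the aggro montage flag is set, trigger AIMoveTo pursuit with cooldown-gated montage attacks and damage on arrival.
; Tick handles the unaware state, stopping movement, resetting the aggro DoOnce and requesting a return to the spawn location saved in the construction script.
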(event OnSeePawn(PawnSensing)
  (params (Pawn :type Pawn%20Object%20Reference))
  (Variables|Default|SetisSeeingPlayer true)
  (Utilities|FlowControl|Sequence
    (:then_0
      ;[1 1 1] Play agro animation once if char is visible (reset value for anim if  char is not visible)
      (Utilities|FlowControl|DoOnce true
        (:Completed
          (bind _returnvalue (Animation|PlayAnimMontage "/Game/Enemies/Animation/AM_Agro.AM_Agro" 1.2 "None"))
          (Utilities|FlowControl|Delay _returnvalue)
          (Variables|Default|SetagroAnimDone true))))
    (:then_1
      (if (Variables|Default|GetagroAnimDone)
        (CallFunction|FollowPlayer)))
    (:then_2
      ;[1 1 1] If char is not seen - reset value
      (Utilities|FlowControl|RetriggerableDelay 1e+01)
      (Variables|Default|SetisSeeingPlayer false))
    (:then_3
      ;[1 1 1] Attack cooldown
      (Utilities|FlowControl|Delay 2.5)
      (Variables|Default|SetcanAttack true))
    (:then_4
      (Variables|Default|SetisInSpawnLocation false))))

(event Custom|Follow%20player
  ;[1 1 1] If player is detected - start following and attacking
  (if (Variables|Default|GetisSeeingPlayer)
    (AI|AIMoveTo self "0, 0, 0" (Game|GetPlayerCharacter 0) 7e+01 false
      (:OnSuccess
        (if (Variables|Default|GetcanAttack)
          (Variables|Default|SetcanAttack false)
          (Animation|PlayAnimMontage "/Game/Enemies/Animation/AM_Attack.AM_Attack" 0.8 "None")
          (Game|Damage|ApplyDamage (Game|GetPlayerCharacter 0) 5.0 0 self "/Script/Engine.DamageType"))))))

(event Custom|MoveBackToSpawn
  ;[1 1 1] Move back to spawn
  (Math|Float|CompareFloat (Math|Float|Absolute(Float) (Math|Vector|VectorLength (- (Variables|Default|GetspawnLocation) (Transformation|GetActorLocation self)))) 1e+01
    (:>
      (AI|AIMoveTo self (Variables|Default|GetspawnLocation) 0 5.0 false
        (:OnSuccess
          (Variables|Default|SetisInSpawnLocation false))))
    (:==
      (Variables|Default|SetisInSpawnLocation true :!label _label))
    (:<
      (goto _label))))

(event EventTick
  (params (DeltaSeconds :type Float%20%28single-precision%29))
  (if (not (Variables|Default|GetisSeeingPlayer))
    (Components|Movement|StopMovementImmediately (Variables|Character|GetCharacterMovement))
    ;[1 1 1] Play agro animation once if char is visible (reset value for anim if  char is not visible)
    (Utilities|FlowControl|Sequence
      (:then_0
        (Variables|Default|SetagroAnimDone false))
      (:then_1
        (Utilities|FlowControl|DoOnce true) ; enters at Reset
      )
      (:then_2
        (if (not (Variables|Default|GetisSeeingPlayer))
          (CallFunction|MoveBacktoSpawn))))))

(event Game|Damage|EventAnyDamage
  (params (Damage :type Float%20%28single-precision%29) (DamageType :type Damage%20Type%20Object%20Reference) (InstigatedBy :type Controller%20Object%20Reference) (DamageCauser :type Actor%20Object%20Reference))
  ;[1 1 1] Take damage
  (bind _output_get (Variables|Default|SetHealth (Math|Float|Truncate (- (Variables|Default|GetHealth) Damage))))
  (Development|PrintString (Utilities|String|ToString(Float) (Math|Conversions|ToFloat(Integer) _output_get)))
  (if (<= (Variables|Default|GetHealth) 0.0)
    (Components|Animation|PlayAnimation (Variables|Character|GetMesh) "/Game/UndeadPack/EnemyGoblin/Animations/Anim_Lose.Anim_Lose" false)
    (Utilities|FlowControl|Delay 5.0)
    (Actor|DestroyActor)))

(fn ConstructionScript
  (Variables|Default|SetspawnLocation (Transformation|GetActorLocation self)))