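; Goblin enemy that wanders around its spawn point, chases and attacks the player, and drops a gold chest on death.
; Event-driven AI without a behavior tree: Tick handles wandering and returning to spawn while the player is unsensed.
; PawnSensing gates pursuit behind a one-time aggro montage, using delays for sight memory and attack cooldown.
; Damage or sphere overlap turns it toward the player through a timeline.
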(event OnSeePawn(PawnSensing)
  (params (Pawn :type Pawn%20Object%20Reference))
  ;[1 1 1] Sense controller
  (if (Variables|Default|GetisAlive)
    (Variables|Default|SetisSensingPlayer true)
    (Utilities|FlowControl|Sequence
      (:then_0
        ;[1 1 1] Play agro animation once if char is visible (reset value for anim if  char is not visible)
        (Utilities|FlowControl|DoOnce true
          (:Completed
            (Components|Movement|StopMovementImmediately (Variables|Character|GetCharacterMovement))
            (bind _returnvalue (Animation|PlayAnimMontage "/Game/Enemies/Animation/Goblin/AM_Agro.AM_Agro" 1.4 "None"))
            (Utilities|FlowControl|Delay _returnvalue)
            (Variables|Default|SetagroAnimDone true))))
      (:then_1
        ;;[1 1 1] If Agro animation was played - follow and attack
        (if (Variables|Default|GetagroAnimDone)
          (CallFunction|FollowPlayer)))
      (:then_2
        ;;[1 1 1] If char is not seen - reset value
        (Utilities|FlowControl|RetriggerableDelay 1e+01)
        (Variables|Default|SetisSensingPlayer false))
      (:then_3
        ;;[1 1 1] Attack cooldown
        (Utilities|FlowControl|Delay 2.5)
        (Variables|Default|SetcanAttack true))
      (:then_4
        ;;[1 1 1] Ped is out of spawn location
        (Variables|Default|SetisInSpawnLocation false)))))

(event OnComponentBeginOverlap(Sphere)
  (params (OverlappedComponent :type Primitive%20Component%20Object%20Reference) (OtherActor :type Actor%20Object%20Reference) (OtherComp :type Primitive%20Component%20Object%20Reference) (OtherBodyIndex :type Integer) (bFromSweep :type Boolean) (SweepResult :type Hit%20Result%20Structure%20%28by%20ref%29))
  ;[1 1 1] Detect player nearby
  (Utilities|Casting|CastToThirdPersonCharacter OtherActor)
  (if (not (Variables|Default|GetisSensingPlayer))
    (CallFunction|SmoothRotatetoTarget)))

(event Custom|Follow%20player
  ;[1 1 1] If player is detected - start following and attacking
  (if (Variables|Default|GetisSensingPlayer)
    (AI|AIMoveTo self "0, 0, 0" (Game|GetPlayerCharacter 0) 2.0 false
      (:OnSuccess
        (if (Variables|Default|GetcanAttack)
          (Variables|Default|SetcanAttack false)
          (Animation|PlayAnimMontage "/Game/Enemies/Animation/Goblin/AM_Attack.AM_Attack" 1.0 "None")
          (Game|Damage|ApplyDamage (Game|GetPlayerCharacter 0) 5.0 0 self "/Script/Engine.DamageType"))))))

(event Custom|Reset%20getting%20random%20location
  ;[1 1 1] When in spawn area & out of combat move freely
  (Utilities|FlowControl|DoOnce false) ; enters at Reset
)

(event Custom|Smooth%20rotate%20to%20target
  ;[1 1 1] Rotate to player character
  (if (Variables|Default|GetisAlive)
    (Variables|Default|SetisSensingPlayer true)
    (Components|Movement|StopMovementImmediately (Variables|Character|GetCharacterMovement))
    (Timeline|Timeline_0 PlayFromStart
      (:Update
        (Transformation|SetActorRelativeRotation (Math|Interpolation|RInterpTo (Transformation|GetActorRotation) (Math|Rotator|MakeRotator 0.0 0.0 (.Yaw (Math|Rotator|BreakRotator (Math|Rotator|FindLookatRotation (Transformation|GetActorLocation) (Transformation|GetActorLocation (Game|GetPlayerCharacter 0)))))) 0.8 0.05))))))

(event Custom|MoveBackToSpawn
  ;[1 1 1] Move back to spawn
  (Math|Float|CompareFloat (Math|Float|Absolute(Float) (Math|Vector|VectorLength (- (Variables|Default|GetspawnLocation) (Transformation|GetActorLocation self)))) 1e+01
    (:>
      (AI|AIMoveTo self (Variables|Default|GetspawnLocation) 0 5.0 false
        (:OnSuccess
          (Variables|Default|SetisInSpawnLocation false))))
    (:==
      (Variables|Default|SetisInSpawnLocation true :!label _label))
    (:<
      (goto _label))))

(event Custom|Reset%20rotation%20command
  ;[1 1 1] Rotate to player character
  (Timeline|Timeline_0 Stop
    (:Update
      (Transformation|SetActorRelativeRotation (Math|Interpolation|RInterpTo (Transformation|GetActorRotation) (Math|Rotator|MakeRotator 0.0 0.0 (.Yaw (Math|Rotator|BreakRotator (Math|Rotator|FindLookatRotation (Transformation|GetActorLocation) (Transformation|GetActorLocation (Game|GetPlayerCharacter 0)))))) 0.8 0.05)))))

(event EventTick
  (params (DeltaSeconds :type Float%20%28single-precision%29))
  (if (Variables|Default|GetisAlive)
    (if (not (Variables|Default|GetisSensingPlayer))
      (Components|Movement|StopMovementImmediately (Variables|Character|GetCharacterMovement))
      ;[1 1 1] Play agro animation once if char is visible (reset value for anim if  char is not visible)
      (Utilities|FlowControl|Sequence
        (:then_0
          (Variables|Default|SetagroAnimDone false))
        (:then_1
          (Utilities|FlowControl|DoOnce true) ; enters at Reset
        )
        (:then_2
          ;[1 1 1] When in spawn area & out of combat move freely
          (if (Variables|Default|GetisInSpawnLocation)
            (Utilities|FlowControl|Sequence
              (:then_0
                (Utilities|FlowControl|DoOnce false
                  (:Completed
                    (bind _randomlocation (Class|NavigationSystemV1|GetRandomLocationinNavigableRadius (Variables|Default|GetspawnLocation) (Variables|Default|GetwanderRadius) 0 0)))))
              (:then_1
                (AI|AIMoveTo self _randomlocation 0 7e+01 false
                  (:OnSuccess
                    (CallFunction|ResetGettingRandomLocation)))))
            (else
              (CallFunction|MoveBacktoSpawn))))))))

(event Game|Damage|EventAnyDamage
  (params (Damage :type Float%20%28single-precision%29) (DamageType :type Damage%20Type%20Object%20Reference) (InstigatedBy :type Controller%20Object%20Reference) (DamageCauser :type Actor%20Object%20Reference))
  ;[1 1 1] Take damage
  (if (Variables|Default|GetisAlive)
    (bind _output_get (Variables|Default|SetHealth (Math|Float|Truncate (- (Variables|Default|GetHealth) Damage))))
    (Development|PrintString (Utilities|String|ToString(Float) (Math|Conversions|ToFloat(Integer) _output_get)))
    (if (<= (Variables|Default|GetHealth) 0.0)
      (Variables|Default|SetisAlive false)
      (CallFunction|ResetRotationCommand)
      (Components|Movement|StopMovementImmediately (Variables|Character|GetCharacterMovement))
      (Components|Animation|PlayAnimation (Variables|Character|GetMesh) "/Game/UndeadPack/EnemyGoblin/Animations/Anim_Lose.Anim_Lose" false)
      (bind _returnvalue (Game|SpawnActorfromClass "/Game/PickupItems/BP_SM_GoldChest.BP_SM_GoldChest_C" (Math|Transform|MakeTransform (Transformation|GetActorLocation)) "Undefined" 0 0))
      (Variables|/Game/PickupItems/BP_SM_GoldChest.BP_SM_GoldChest_C|SetgoldToAdd _returnvalue (Variables|Default|GetgoldToDrop))
      (Utilities|FlowControl|Delay 5.0)
      (Actor|DestroyActor)
      (else
        (CallFunction|SmoothRotatetoTarget)))))

(fn ConstructionScript
  (Variables|Default|SetspawnLocation (Transformation|GetActorLocation self)))