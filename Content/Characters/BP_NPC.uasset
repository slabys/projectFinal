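; BP_NPC is an NPC Blueprint that steps through lines of dialogue in a WB_dialog widget.
; Each Talk call increments ChatIndex and writes that Chat entry to the widget's Dialogue text.
; The widget is created for player controller 0 and added to the viewport only when the UI reference is invalid.
; Past the last line it is removed from its parent, and the index is not reset here.
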(event EventTalk
  (Math|Integer|IncrementInt (Variables|Default|GetchatIndex)
    (:%20%20
      (if (< (Variables|Default|GetchatIndex) (Utilities|Array|Length (Variables|Default|Getchat)))
        (Variables|Default|GetUI
          (:then
            _)
          (:else
            (bind _returnvalue (UserInterface|CreateWidget "/Game/Characters/DialogInterface/WB_dialog.WB_dialog_C" (Game|GetPlayerController 0)))
            (bind _output_get (Variables|Default|SetUI _returnvalue))
            (UserInterface|Viewport|AddtoViewport _output_get 0)))
        (Rendering|Components|TextRender|SetText (Variables|/Game/Characters/DialogInterface/WB_dialog.WB_dialog_C|Getdialogue (Variables|Default|GetUI)) (Utilities|Text|ToText(String) (Utilities|Array|Get(acopy) (Variables|Default|Getchat) (Variables|Default|GetchatIndex))))
        (else
          (Widget|RemovefromParent (Variables|Default|GetUI)))))))

(fn ConstructionScript)