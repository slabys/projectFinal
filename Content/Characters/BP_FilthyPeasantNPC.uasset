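; Peasant NPC that wanders around its spawn area and complains when hurt.
; Tick picks a random navigable point within WanderRadius of SpawnLocation when idle and calls AIMoveTo every frame, clearing IsMoving only on success.
; Any damage shows a line of text on the TextAbove widget, then hides it after a delay.
; The F key handler loops over overlapping actors but does nothing with them.
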(event EventBeginPlay)

(event Collision|EventActorBeginOverlap
  (params (OtherActor :type Actor%20Object%20Reference)))

(event EventTick
  (params (DeltaSeconds :type Float%20%28single-precision%29))
  (if (Variables|Default|GetisMoving)
    _
    (else
      (bind _randomlocation (Class|NavigationSystemV1|GetRandomLocationinNavigableRadius (Variables|Default|GetspawnLocation) (Variables|Default|GetwanderRadius) 0 0))
      (Variables|Default|SetisMoving true)))
  (AI|AIMoveTo self _randomlocation 0 3e+01 false
    (:OnSuccess
      (Variables|Default|SetisMoving false))))

(event Game|Damage|EventAnyDamage
  (params (Damage :type Float%20%28single-precision%29) (DamageType :type Damage%20Type%20Object%20Reference) (InstigatedBy :type Controller%20Object%20Reference) (DamageCauser :type Actor%20Object%20Reference))
  (bind _astext_above (Utilities|Casting|CastToTextAbove (UserInterface|GetUserWidgetObject (Variables|Default|GetWidget))))
  (Widget|SetVisibility (Variables|/Game/Characters/UI/TextAbove.TextAbove_C|GetTextAboveCharacter _astext_above) "Visible")
  (Rendering|Components|TextRender|SetText (Variables|/Game/Characters/UI/TextAbove.TextAbove_C|GetTextAboveCharacter _astext_above) "Why is everyone so evil these days?")
  (Utilities|FlowControl|Delay 1e+01)
  (Widget|SetVisibility (Variables|/Game/Characters/UI/TextAbove.TextAbove_C|GetTextAboveCharacter _astext_above) "Hidden"))

(event Input|KeyboardEvents|F
  (params (Key :type Key%20Structure :default "None"))
  (:Pressed
    (for _array_element (Collision|GetOverlappingActors 0 :!class /Script/Engine.Actor)
      _)))

(fn ConstructionScript)