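; BP_Barrel is a map prop that shows a joke comment about selling booze when the main character walks up to it.
; Entering BarrelTrigger reveals the TextAbove widget on the BarrelComment component and sets its text to a hardcoded line.
; Leaving the trigger hides the widget after a fixed delay, which re-entering does not cancel.
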(event OnComponentBeginOverlap(BarrelTrigger)
  (params (OverlappedComponent :type Primitive%20Component%20Object%20Reference) (OtherActor :type Actor%20Object%20Reference) (OtherComp :type Primitive%20Component%20Object%20Reference) (OtherBodyIndex :type Integer) (bFromSweep :type Boolean) (SweepResult :type Hit%20Result%20Structure%20%28by%20ref%29))
  (Utilities|Casting|CastToMainCharacter OtherActor)
  (bind _astext_above (Utilities|Casting|CastToTextAbove (UserInterface|GetUserWidgetObject (Variables|Default|GetBarrelComment))))
  (Widget|SetVisibility _astext_above "Visible")
  (Rendering|Components|TextRender|SetText (Variables|/Game/Characters/UI/TextAbove.TextAbove_C|GetTextAboveCharacter _astext_above) "Holy fu**, I could make fortune by selling this booze"))

(event OnComponentEndOverlap(BarrelTrigger)
  (params (OverlappedComponent :type Primitive%20Component%20Object%20Reference) (OtherActor :type Actor%20Object%20Reference) (OtherComp :type Primitive%20Component%20Object%20Reference) (OtherBodyIndex :type Integer))
  (Utilities|Casting|CastToMainCharacter OtherActor)
  (bind _astext_above (Utilities|Casting|CastToTextAbove (UserInterface|GetUserWidgetObject (Variables|Default|GetBarrelComment))))
  (Utilities|FlowControl|Delay 1e+01)
  (Widget|SetVisibility _astext_above "Hidden"))

(fn ConstructionScript)