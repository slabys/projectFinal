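; An outhouse prop Blueprint that shows a random line of flavour text when the player character walks into it.
; Overlapping its collision box with MainCharacter sets a random entry from TextToShow on the TextAbove widget component and makes it visible.
; A DoOnce gate blocks retriggers until the text hides again after a short delay.
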(event OnComponentBeginOverlap(CollisionBox)
  (params (OverlappedComponent :type Primitive%20Component%20Object%20Reference) (OtherActor :type Actor%20Object%20Reference) (OtherComp :type Primitive%20Component%20Object%20Reference) (OtherBodyIndex :type Integer) (bFromSweep :type Boolean) (SweepResult :type Hit%20Result%20Structure%20%28by%20ref%29))
  (Utilities|Casting|CastToMainCharacter OtherActor)
  (bind _astext_above (Utilities|Casting|CastToTextAbove (UserInterface|GetUserWidgetObject (Variables|Default|GetWidget))))
  (Utilities|FlowControl|DoOnce false :!label _label
    (:Completed
      (Widget|SetVisibility (Variables|/Game/Characters/UI/TextAbove.TextAbove_C|GetTextAboveCharacter _astext_above) "Visible")
      (Rendering|Components|TextRender|SetText (Variables|/Game/Characters/UI/TextAbove.TextAbove_C|GetTextAboveCharacter _astext_above) (Utilities|Text|ToText(String) (.OutItem (Utilities|Array|Random (Variables|Default|GetTextToShow)))))
      (Utilities|FlowControl|Delay 5.0)
      (Widget|SetVisibility (Variables|/Game/Characters/UI/TextAbove.TextAbove_C|GetTextAboveCharacter _astext_above) "Hidden")
      (goto _label Reset))))

(fn ConstructionScript)